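; BP_LevelManager is a level manager that tracks an ingredient count and switches bartender dialogue actors once at least three are counted.
; The count resets to zero on BeginPlay and is only read here, not incremented.
; Tick polls it and, at the threshold, looks up the first dialogue actor to call Hidden, then the second to call Active.
; There is no one-shot guard, so this repeats every frame while both actors remain valid.
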(event `self.ReceiveBeginPlay`
  (set `self.Ingredients` 0))

(event `self.ReceiveTick`
  (params (DeltaSeconds :type "Float (single-precision)"))
  (if (>= (`self.Ingredients`) 3)
    (bind _returnvalue (`GameplayStatics.GetActorOfClass` "/Game/BetweenTheLines/Interactables/BP_Dialogues/BP_Dialogues/BP_BartendeDialogueChildr.BP_BartendeDialogueChildr_C"))
    (`/Engine/EditorBlueprintResources/StandardMacros.IsValid` _returnvalue
      (:`Is Valid`
        (`/Game/BetweenTheLines/Interactables/BP_Dialogues/BP_Dialogues/BP_BartendeDialogueChildr.Hidden` _returnvalue)
        (bind _returnvalue_2 (`GameplayStatics.GetActorOfClass` "/Game/BetweenTheLines/Interactables/BP_Dialogues/BP_Dialogues/BP_BartendeDialogueChildr2.BP_BartendeDialogueChildr2_C"))
        (`/Engine/EditorBlueprintResources/StandardMacros.IsValid` _returnvalue_2
          (:`Is Valid`
            (`/Game/BetweenTheLines/Interactables/BP_Dialogues/BP_Dialogues/BP_BartendeDialogueChildr2.Active` _returnvalue_2)))))))

(fn `UserConstructionScript`)