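; BP_WireMinigame is a Level 1 interactable actor that opens the wire minigame when interacted with.
; On OnInteract it creates a WB_WireMinigame widget for the first player controller and adds it to the viewport.
; It then switches input to UI-only focused on that widget, shows the mouse cursor and sets permanent mouse capture.
; The blueprint only launches the UI and holds no puzzle logic or code to restore game input.
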(event `/Game/BetweenTheLines/Interaction/IInteractable.OnInteract`
  (bind _returnvalue (`|CreateWidget` "/Game/BetweenTheLines/UI/Blueprints/Minigames/Football_Zone/WB_WireMinigame.WB_WireMinigame_C" (`GameplayStatics.GetPlayerController` 0)))
  (`UserWidget.AddToViewport` _returnvalue 0)
  (`WidgetBlueprintLibrary.SetInputMode_UIOnlyEx` (`GameplayStatics.GetPlayerController` 0) _returnvalue)
  (set `PlayerController.bShowMouseCursor` true (`GameplayStatics.GetPlayerController` 0))
  (`GameplayStatics.SetViewportMouseCaptureMode` "CapturePermanently"))

(fn `UserConstructionScript`
  (`parent.UserConstructionScript`))