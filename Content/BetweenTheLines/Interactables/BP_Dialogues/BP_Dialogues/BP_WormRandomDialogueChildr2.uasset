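; Worm dialogue interactable that starts hidden, with collision and tick disabled until something outside this Blueprint enables it.
; Each interaction locks player movement and advances through the dialogue lines in a WB_Dialogue widget, swapping to a spider portrait for the second and third lines.
; When the lines run out, it closes the widget, restores walking and activates the BP_BabySpiderRandomDialogueChildr actor, chaining to the next conversation.
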(event `self.ReceiveBeginPlay`
  (`parent.ReceiveBeginPlay`)
  (`self.SetActorHiddenInGame` true)
  (`self.SetActorEnableCollision` false)
  (`self.SetActorTickEnabled` false))

(event `self.DialogueFunction`
  (`self.UI Ref`
    (:`then`
      (if (or (== (`self.TalkIndex`) 1) (== (`self.TalkIndex`) 2))
        (`/Game/BetweenTheLines/UI/Blueprints/Dialogue/WB_Dialogue.Set Portrait` (`self.UI Ref`) (`self.SpiderPNG`))
        (else
          (`/Game/BetweenTheLines/UI/Blueprints/Dialogue/WB_Dialogue.Set Portrait` (`self.UI Ref`) (`self.PortraitPNG`)))))
    (:`else`
      (bind _returnvalue (`|CreateWidget` "/Game/BetweenTheLines/UI/Blueprints/Dialogue/WB_Dialogue.WB_Dialogue_C" (`GameplayStatics.GetPlayerController` 0)))
      (bind _output_get (set `self.UI Ref` _returnvalue))
      (`UserWidget.AddToViewport` _output_get 0)
      (if (or (== (`self.TalkIndex`) 1) (== (`self.TalkIndex`) 2))
        (`/Game/BetweenTheLines/UI/Blueprints/Dialogue/WB_Dialogue.Set Portrait` (`self.UI Ref`) (`self.SpiderPNG`))
        (else
          (`/Game/BetweenTheLines/UI/Blueprints/Dialogue/WB_Dialogue.Set Portrait` (`self.UI Ref`) (`self.PortraitPNG`))))))
  (`TextBlock.SetText` (`/Game/BetweenTheLines/UI/Blueprints/Dialogue/WB_Dialogue.DialogueText` (`self.UI Ref`)) (`KismetTextLibrary.Conv_StringToText` (`|GetArrayItem` (`self.Dialogue`) (`self.TalkIndex`)))))

(event `self.ReceiveTick`
  (params (DeltaSeconds :type "Float (single-precision)"))
  (`parent.ReceiveTick` DeltaSeconds))

(event `self.OnInteract`
  (`SceneComponent.SetHiddenInGame` (`self.CanDialogueWidget`) true false)
  (set `self.AfterInteraction` true)
  (`CharacterMovementComponent.DisableMovement` (`Character.CharacterMovement` (`self.PlayerRef`)))
  (`SceneComponent.SetHiddenInGame` (`self.Widget`) false false)
  (`/Engine/EditorBlueprintResources/StandardMacros.IncrementInt` (`self.TalkIndex`)
    (:`  `
      (if (< (`self.TalkIndex`) (`KismetArrayLibrary.Array_Length` (`self.Dialogue`)))
        (`self.DialogueFunction`)
        (else
          (`/Game/BetweenTheLines/UI/Blueprints/Dialogue/WB_Dialogue.DestroyDialogue` (`self.UI Ref`))
          (`CharacterMovementComponent.SetMovementMode` (`Character.CharacterMovement` (`self.PlayerRef`)) "MOVE_Walking" 0)
          (set `self.TalkIndex` -1)
          (set `self.UI Ref` null)
          (`SceneComponent.SetHiddenInGame` (`self.CanDialogueWidget`) true false)
          (bind _returnvalue (`GameplayStatics.GetActorOfClass` "/Game/BetweenTheLines/Interactables/BP_Dialogues/BP_Dialogues/BP_BabySpiderRandomDialogueChildr.BP_BabySpiderRandomDialogueChildr_C"))
          (`self.SetActorHiddenInGame` _returnvalue false)
          (`self.SetActorTickEnabled` _returnvalue true)
          (`self.SetActorEnableCollision` _returnvalue true))))))

(fn `Hidden`
  (`self.SetActorHiddenInGame` true)
  (`self.K2_DestroyActor`))

(fn `UserConstructionScript`
  (`parent.UserConstructionScript`))