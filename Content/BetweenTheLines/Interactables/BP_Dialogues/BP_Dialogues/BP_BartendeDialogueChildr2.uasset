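; Second bartender dialogue interactable, a child Blueprint that stays hidden, non-ticking and non-colliding from BeginPlay until Active is called.
; Each interaction locks player movement and advances TalkIndex through the inherited Dialogue lines.
; After the last line it destroys the dialogue UI, restores walking and resets the index.
; It then unlocks the next step by enabling the spider panel's widget and collision and the scarab random dialogue's collision.
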(event `self.ReceiveBeginPlay`
  (`parent.ReceiveBeginPlay`)
  (`self.SetActorHiddenInGame` true)
  (`self.SetActorTickEnabled` false)
  (`self.SetActorEnableCollision` false))

(event `self.ReceiveTick`
  (params (DeltaSeconds :type "Float (single-precision)"))
  (`parent.ReceiveTick` DeltaSeconds))

(event `self.OnInteract`
  (`SceneComponent.SetHiddenInGame` (`self.CanDialogueWidget`) true false)
  (set `self.AfterInteraction` true)
  (`CharacterMovementComponent.DisableMovement` (`Character.CharacterMovement` (`self.PlayerRef`)))
  (`SceneComponent.SetHiddenInGame` (`self.Widget`) false false)
  (`/Engine/EditorBlueprintResources/StandardMacros.IncrementInt` (`self.TalkIndex`)
    (:`  `
      (if (< (`self.TalkIndex`) (`KismetArrayLibrary.Array_Length` (`self.Dialogue`)))
        (`self.DialogueFunction`)
        (else
          (`/Game/BetweenTheLines/UI/Blueprints/Dialogue/WB_Dialogue.DestroyDialogue` (`self.UI Ref`))
          (`CharacterMovementComponent.SetMovementMode` (`Character.CharacterMovement` (`self.PlayerRef`)) "MOVE_Walking" 0)
          (set `self.TalkIndex` -1)
          (set `self.UI Ref` null)
          (`SceneComponent.SetHiddenInGame` (`self.CanDialogueWidget`) true false)
          (bind _returnvalue (`GameplayStatics.GetActorOfClass` "/Game/BetweenTheLines/Interactables/Level_1/BP_InteractableParentSpiderPanel.BP_InteractableParentSpiderPanel_C"))
          (`SceneComponent.SetHiddenInGame` (`/Game/BetweenTheLines/Interactables/BP_Parent/BP_InteractableParentSpider.Widget` _returnvalue) false false)
          (`self.SetActorEnableCollision` _returnvalue true)
          (bind _returnvalue_2 (`GameplayStatics.GetActorOfClass` "/Game/BetweenTheLines/Interactables/BP_Dialogues/BP_Dialogues/BP_ScarabRandomDialogueChildr1.BP_ScarabRandomDialogueChildr1_C"))
          (`self.SetActorEnableCollision` _returnvalue_2 true))))))

(fn `Active`
  (`self.SetActorHiddenInGame` false)
  (`self.SetActorTickEnabled` true)
  (`self.SetActorEnableCollision` true))

(fn `UserConstructionScript`
  (`parent.UserConstructionScript`))