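; Scarab dialogue interactable, a child Blueprint that starts with actor collision disabled and steps through the lines of an inherited dialogue system.
; Each OnInteract freezes player movement, swaps the prompt widget for the dialogue widget, and advances TalkIndex through the Dialogue array via DialogueFunction.
; Past the last line it destroys the dialogue UI, restores walking and resets the index.
; A separate Hidden function hides and destroys the actor.
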(event `self.ReceiveBeginPlay`
  (`parent.ReceiveBeginPlay`)
  (`self.SetActorEnableCollision` false))

(event `self.ReceiveTick`
  (params (DeltaSeconds :type "Float (single-precision)"))
  (`parent.ReceiveTick` DeltaSeconds))

(event `self.OnInteract`
  (`SceneComponent.SetHiddenInGame` (`self.CanDialogueWidget`) true false)
  (set `self.AfterInteraction` true)
  (`CharacterMovementComponent.DisableMovement` (`Character.CharacterMovement` (`self.PlayerRef`)))
  (`SceneComponent.SetHiddenInGame` (`self.Widget`) false false)
  (`/Engine/EditorBlueprintResources/StandardMacros.IncrementInt` (`self.TalkIndex`)
    (:`  `
      (if (< (`self.TalkIndex`) (`KismetArrayLibrary.Array_Length` (`self.Dialogue`)))
        (`self.DialogueFunction`)
        (else
          (`/Game/BetweenTheLines/UI/Blueprints/Dialogue/WB_Dialogue.DestroyDialogue` (`self.UI Ref`))
          (`CharacterMovementComponent.SetMovementMode` (`Character.CharacterMovement` (`self.PlayerRef`)) "MOVE_Walking" 0)
          (set `self.TalkIndex` -1)
          (set `self.UI Ref` null)
          (`SceneComponent.SetHiddenInGame` (`self.CanDialogueWidget`) true false))))))

(fn `Hidden`
  (`self.SetActorHiddenInGame` true)
  (`self.K2_DestroyActor`))

(fn `UserConstructionScript`
  (`parent.UserConstructionScript`))