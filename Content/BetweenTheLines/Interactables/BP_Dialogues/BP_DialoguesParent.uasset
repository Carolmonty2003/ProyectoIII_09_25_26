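; Parent Blueprint for interactable dialogue actors that show lines of text on screen as the player interacts.
; OnInteract hides the actor's Widget component, then, if TalkIndex is within or equal to the Dialogue array's length, waits briefly and increments the index.
; It creates a WB_Dialogue widget when none is valid, reuses it afterwards, and sets its text to the entry at the new index.
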(event `/Game/BetweenTheLines/Interaction/IInteractable.OnInteract`
  (`SceneComponent.SetHiddenInGame` (`self.Widget`) true false)
  (if (<= (`self.TalkIndex`) (`KismetArrayLibrary.Array_Length` (`self.Dialogue`)))
    (`KismetSystemLibrary.Delay` 1.0)
    (`/Engine/EditorBlueprintResources/StandardMacros.IncrementInt` (`self.TalkIndex`)
      (:`  `
        (`self.UI`
          (:`then`
            _)
          (:`else`
            (bind _returnvalue (`|CreateWidget` "/Game/BetweenTheLines/UI/Blueprints/Dialogue/WB_Dialogue.WB_Dialogue_C" (`GameplayStatics.GetPlayerController` 0)))
            (bind _output_get (set `self.UI` _returnvalue))
            (`UserWidget.AddToViewport` _output_get 0)))
        (`TextBlock.SetText` (`/Game/BetweenTheLines/UI/Blueprints/Dialogue/WB_Dialogue.DialogueText` (`self.UI`)) (`KismetTextLibrary.Conv_StringToText` (`|GetArrayItem` (`self.Dialogue`) (`self.TalkIndex`))))))))

(fn `UserConstructionScript`
  (`parent.UserConstructionScript`))