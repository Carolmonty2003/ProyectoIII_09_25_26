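; BP_InteractableParent is a base interactable actor that detects when the BP_ThirdPersonEscriba player character is within range.
; On sphere overlap it stores the player and registers itself as that character's CurrentInteractable, enabling custom depth on its mesh and showing its widget.
; Leaving the sphere clears both references, disables custom depth and hides the widget.
; This graph contains no interaction logic itself, only proximity registration and visual feedback.
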(event `self.Sphere.OnComponentBeginOverlap`
  (params (OverlappedComponent :type "PrimitiveComponent Object Reference") (OtherActor :type "Actor Object Reference") (OtherComp :type "PrimitiveComponent Object Reference") (OtherBodyIndex :type Integer) (bFromSweep :type Boolean) (SweepResult :type "HitResult Structure (by ref)"))
  (bind _asbp_third_person_escriba (cast `/Game/BetweenTheLines/Characters/EscribaCharacter/Blueprints/BP_ThirdPersonEscriba` OtherActor))
  (set `self.PlayerRef` _asbp_third_person_escriba)
  (set `/Game/BetweenTheLines/Characters/EscribaCharacter/Blueprints/BP_ThirdPersonEscriba.CurrentInteractable` self _asbp_third_person_escriba)
  (`PrimitiveComponent.SetRenderCustomDepth` (`self.StaticMesh`) true)
  (`SceneComponent.SetHiddenInGame` (`self.Widget`) false false))

(event `self.Sphere.OnComponentEndOverlap`
  (params (OverlappedComponent :type "PrimitiveComponent Object Reference") (OtherActor :type "Actor Object Reference") (OtherComp :type "PrimitiveComponent Object Reference") (OtherBodyIndex :type Integer))
  (bind _asbp_third_person_escriba (cast `/Game/BetweenTheLines/Characters/EscribaCharacter/Blueprints/BP_ThirdPersonEscriba` OtherActor))
  (set `self.PlayerRef` null)
  (set `/Game/BetweenTheLines/Characters/EscribaCharacter/Blueprints/BP_ThirdPersonEscriba.CurrentInteractable` null _asbp_third_person_escriba)
  (`PrimitiveComponent.SetRenderCustomDepth` (`self.StaticMesh`) false)
  (`SceneComponent.SetHiddenInGame` (`self.Widget`) true false))

(fn `UserConstructionScript`)