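; Parent Blueprint for interactable dialogue actors, showing floating text when the spider player character enters range.
; Each OnInteract advances through the Dialogue array in a lazily created WB_Dialogue widget while player movement is disabled.
; After the last line it destroys the dialogue, restores walking and resets the index for replay.
; The first interaction permanently suppresses the floating text and hides the other Widget component.
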(event `/Game/BetweenTheLines/Interaction/IInteractable.OnInteract`
  (`SceneComponent.SetHiddenInGame` (`self.CanDialogueWidget`) true false)
  (set `self.AfterInteraction` true)
  (`CharacterMovementComponent.DisableMovement` (`Character.CharacterMovement` (`self.PlayerRef`)))
  (`SceneComponent.SetHiddenInGame` (`self.Widget`) true false)
  (`/Engine/EditorBlueprintResources/StandardMacros.IncrementInt` (`self.TalkIndex`)
    (:`  `
      (if (< (`self.TalkIndex`) (`KismetArrayLibrary.Array_Length` (`self.Dialogue`)))
        (`self.DialogueFunction`)
        (else
          (`/Game/BetweenTheLines/UI/Blueprints/Dialogue/WB_Dialogue.DestroyDialogue` (`self.UI Ref`))
          (`CharacterMovementComponent.SetMovementMode` (`Character.CharacterMovement` (`self.PlayerRef`)) "MOVE_Walking" 0)
          (set `self.TalkIndex` -1)
          (set `self.UI Ref` null))))))

(event `self.CanDialogue.OnComponentBeginOverlap`
  (params (OverlappedComponent :type "PrimitiveComponent Object Reference") (OtherActor :type "Actor Object Reference") (OtherComp :type "PrimitiveComponent Object Reference") (OtherBodyIndex :type Integer) (bFromSweep :type Boolean) (SweepResult :type "HitResult Structure (by ref)"))
  (cast `/Game/BetweenTheLines/Characters/SpiderCharacter/blueprints/BP_ThirdPersonSpider` OtherActor)
  (if (not (`self.AfterInteraction`))
    (`SceneComponent.SetHiddenInGame` (`self.CanDialogueWidget`) false false)
    (`self.FloatingTextFunction`)))

(event `self.CanDialogue.OnComponentEndOverlap`
  (params (OverlappedComponent :type "PrimitiveComponent Object Reference") (OtherActor :type "Actor Object Reference") (OtherComp :type "PrimitiveComponent Object Reference") (OtherBodyIndex :type Integer))
  (cast `/Game/BetweenTheLines/Characters/SpiderCharacter/blueprints/BP_ThirdPersonSpider` OtherActor)
  (`SceneComponent.SetHiddenInGame` (`self.CanDialogueWidget`) true false))

(fn `DialogueFunction`
  (`self.UI Ref`
    (:`then`
      _)
    (:`else`
      (bind _returnvalue (`|CreateWidget` "/Game/BetweenTheLines/UI/Blueprints/Dialogue/WB_Dialogue.WB_Dialogue_C" (`GameplayStatics.GetPlayerController` 0)))
      (bind _output_get (set `self.UI Ref` _returnvalue))
      (`UserWidget.AddToViewport` _output_get 0)))
  (`TextBlock.SetText` (`/Game/BetweenTheLines/UI/Blueprints/Dialogue/WB_Dialogue.DialogueText` (`self.UI Ref`)) (`KismetTextLibrary.Conv_StringToText` (`|GetArrayItem` (`self.Dialogue`) (`self.TalkIndex`)))))

(fn `FloatingTextFunction`
  (`TextBlock.SetText` (`/Game/BetweenTheLines/UI/Blueprints/Dialogue/WB_FloatingText.FloatingText` (cast `/Game/BetweenTheLines/UI/Blueprints/Dialogue/WB_FloatingText` (`WidgetComponent.GetUserWidgetObject` (`self.CanDialogueWidget`)) :!pure true)) (`KismetTextLibrary.Conv_StringToText` (`self.FloatingText`))))

(fn `UserConstructionScript`
  (`parent.UserConstructionScript`))