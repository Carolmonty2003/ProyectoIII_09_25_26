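; Parent Blueprint for interactables that show a sequence of dialogue lines as the player interacts with them.
; Each OnInteract disables player movement, hides the Widget component and advances TalkIndex through the Dialogue array.
; DialogueFunction creates the dialogue UI if none is valid and sets its text to the current line.
; After the last line, it destroys the UI, restores walking and resets the index, allowing replay.
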(event `/Game/BetweenTheLines/Interaction/IInteractable.OnInteract`
  (`CharacterMovementComponent.DisableMovement` (`Character.CharacterMovement` (`self.PlayerRef`)))
  (`SceneComponent.SetHiddenInGame` (`self.Widget`) true false)
  (`/Engine/EditorBlueprintResources/StandardMacros.IncrementInt` (`self.TalkIndex`)
    (:`  `
      (if (< (`self.TalkIndex`) (`KismetArrayLibrary.Array_Length` (`self.Dialogue`)))
        (`self.DialogueFunction`)
        (else
          (`/Game/BetweenTheLines/UI/Blueprints/Dialogue/WB_Dialogue.DestroyDialogue` (`self.UIRef`))
          (`CharacterMovementComponent.SetMovementMode` (`Character.CharacterMovement` (`self.PlayerRef`)) "MOVE_Walking" 0)
          (set `self.TalkIndex` -1)
          (set `self.UIRef` null))))))

(fn `DialogueFunction`
  (`self.UIRef`
    (:`then`
      _)
    (:`else`
      (bind _returnvalue (`|CreateWidget` "/Game/BetweenTheLines/UI/Blueprints/Dialogue/WB_Dialogue.WB_Dialogue_C" (`GameplayStatics.GetPlayerController` 0)))
      (bind _output_get (set `self.UIRef` _returnvalue))
      (`UserWidget.AddToViewport` _output_get 0)))
  (`TextBlock.SetText` (`/Game/BetweenTheLines/UI/Blueprints/Dialogue/WB_Dialogue.DialogueText` (`self.UIRef`)) (`KismetTextLibrary.Conv_StringToText` (`|GetArrayItem` (`self.Dialogue`) (`self.TalkIndex`)))))

(fn `UserConstructionScript`
  (`parent.UserConstructionScript`))