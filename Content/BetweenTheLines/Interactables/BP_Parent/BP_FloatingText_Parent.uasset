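; Parent Blueprint for interactable floating text that appears when the BP_ThirdPersonEscriba player character comes near.
; A sphere's begin and end overlap events show and hide a widget component, ignoring any other actor.
; On each show, FloatingTextFunction copies the Text variable into the FloatingText field of the WB_FloatingText widget.
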(event `self.Sphere.OnComponentBeginOverlap`
  (params (OverlappedComponent :type "PrimitiveComponent Object Reference") (OtherActor :type "Actor Object Reference") (OtherComp :type "PrimitiveComponent Object Reference") (OtherBodyIndex :type Integer) (bFromSweep :type Boolean) (SweepResult :type "HitResult Structure (by ref)"))
  (cast `/Game/BetweenTheLines/Characters/EscribaCharacter/Blueprints/BP_ThirdPersonEscriba` OtherActor)
  (`SceneComponent.SetHiddenInGame` (`self.Widget`) false false)
  (`self.FloatingTextFunction`))

(event `self.Sphere.OnComponentEndOverlap`
  (params (OverlappedComponent :type "PrimitiveComponent Object Reference") (OtherActor :type "Actor Object Reference") (OtherComp :type "PrimitiveComponent Object Reference") (OtherBodyIndex :type Integer))
  (cast `/Game/BetweenTheLines/Characters/EscribaCharacter/Blueprints/BP_ThirdPersonEscriba` OtherActor)
  (`SceneComponent.SetHiddenInGame` (`self.Widget`) true false))

(fn `FloatingTextFunction`
  (`TextBlock.SetText` (`/Game/BetweenTheLines/UI/Blueprints/Dialogue/WB_FloatingText.FloatingText` (cast `/Game/BetweenTheLines/UI/Blueprints/Dialogue/WB_FloatingText` (`WidgetComponent.GetUserWidgetObject` (`self.Widget`)) :!pure true)) (`KismetTextLibrary.Conv_StringToText` (`self.Text`))))

(fn `UserConstructionScript`)