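; BP_DeadBox is a kill volume in Level 1 that sends the spider player back to the last checkpoint on overlap.
; When BP_ThirdPersonSpider enters the box, it disables input and teleports the spider to the checkpoint location stored in GameInstanceBetweenTheLines, with zero rotation.
; It then stops the player character's movement immediately to clear momentum and re-enables input.
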(event `self.Box.OnComponentBeginOverlap`
  (params (OverlappedComponent :type "PrimitiveComponent Object Reference") (OtherActor :type "Actor Object Reference") (OtherComp :type "PrimitiveComponent Object Reference") (OtherBodyIndex :type Integer) (bFromSweep :type Boolean) (SweepResult :type "HitResult Structure (by ref)"))
  (bind _asbp_third_person_spider (cast `/Game/BetweenTheLines/Characters/SpiderCharacter/blueprints/BP_ThirdPersonSpider` OtherActor))
  (`self.DisableInput` _asbp_third_person_spider (`GameplayStatics.GetPlayerController` 0))
  (bind _asgame_instance_between_the_lines (cast `/Game/BetweenTheLines/GameInstanceBetweenTheLines` (`GameplayStatics.GetGameInstance`)))
  (`self.K2_TeleportTo` :`self` _asbp_third_person_spider :`DestLocation` (`/Game/BetweenTheLines/GameInstanceBetweenTheLines.LastChekPointLocation` _asgame_instance_between_the_lines))
  (`MovementComponent.StopMovementImmediately` (`Character.CharacterMovement` (`GameplayStatics.GetPlayerCharacter` 0)))
  (`self.EnableInput` _asbp_third_person_spider (`GameplayStatics.GetPlayerController` 0)))

(fn `UserConstructionScript`)