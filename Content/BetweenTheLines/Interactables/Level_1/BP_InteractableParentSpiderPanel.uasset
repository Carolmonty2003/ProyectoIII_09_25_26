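; Level 1 interactable spider panel pickup that advances the police dialogue when taken.
; It starts with its widget hidden and collision disabled; nothing in this file re-enables that collision.
; On interact it sets the ItTakeIt flag and hides itself, then destroys BP_PoliceDialogueChild and reveals BP_PoliceDialogueChild2 with tick and collision enabled.
; The panel then destroys itself.
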(event `self.ReceiveBeginPlay`
  (`parent.ReceiveBeginPlay`)
  (`SceneComponent.SetHiddenInGame` (`self.Widget`) true false)
  (`self.SetActorEnableCollision` false))

(event `/Game/BetweenTheLines/Interaction/IInteractable.OnInteract`
  (set `self.itTakeIt` true)
  (`self.SetActorHiddenInGame` true)
  (bind _returnvalue (`GameplayStatics.GetActorOfClass` "/Game/BetweenTheLines/Interactables/BP_Dialogues/BP_Dialogues/BP_PoliceDialogueChild.BP_PoliceDialogueChild_C"))
  (`self.SetActorHiddenInGame` _returnvalue true)
  (`self.K2_DestroyActor` _returnvalue)
  (bind _returnvalue_2 (`GameplayStatics.GetActorOfClass` "/Game/BetweenTheLines/Interactables/BP_Dialogues/BP_Dialogues/BP_PoliceDialogueChild2.BP_PoliceDialogueChild2_C"))
  (`self.SetActorHiddenInGame` _returnvalue_2 false)
  (`self.SetActorTickEnabled` _returnvalue_2 true)
  (`self.SetActorEnableCollision` _returnvalue_2 true)
  (`self.K2_DestroyActor`))

(fn `UserConstructionScript`
  (`parent.UserConstructionScript`))