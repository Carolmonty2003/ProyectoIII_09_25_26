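; Base interactable for collectible ingredients in Level 1.
; On BeginPlay it hides itself and turns off tick and collision, and contains no logic to re-enable them.
; When OnInteract fires, it finds BP_LevelManager with GetActorOfClass, increments its Ingredients count and destroys itself.
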(event `self.ReceiveBeginPlay`
  (`parent.ReceiveBeginPlay`)
  (`self.SetActorHiddenInGame` true)
  (`self.SetActorTickEnabled` false)
  (`self.SetActorEnableCollision` false))

(event `/Game/BetweenTheLines/Interaction/IInteractable.OnInteract`
  (bind _returnvalue (`GameplayStatics.GetActorOfClass` "/Game/BetweenTheLines/BP_LevelManager.BP_LevelManager_C"))
  (set `/Game/BetweenTheLines/BP_LevelManager.Ingredients` (+ (`/Game/BetweenTheLines/BP_LevelManager.Ingredients` _returnvalue) 1) _returnvalue)
  (`self.K2_DestroyActor`))

(fn `UserConstructionScript`
  (`parent.UserConstructionScript`))