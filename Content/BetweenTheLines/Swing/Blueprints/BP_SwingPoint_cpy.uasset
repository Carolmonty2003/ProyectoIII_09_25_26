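; Projectile swing point for the spider character's grapple, apparently a copy of another swing point Blueprint.
; On BeginPlay it caches the player's BP_ThirdPersonSpider, applies its Velocity to the projectile movement and records its start location.
; When the static mesh hits something, it switches the spider's grapple state and stores the sphere's world location as the hooked location.
; GetArcPoints only returns a stored arc point variable.
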(event `self.ReceiveBeginPlay`
  (bind _asbp_third_person_spider (cast `/Game/BetweenTheLines/Characters/SpiderCharacter/blueprints/BP_ThirdPersonSpider` (`GameplayStatics.GetPlayerPawn` 0)))
  (set `self.As BP Third Person Spider` _asbp_third_person_spider)
  (set `MovementComponent.Velocity` (`self.Velocity`) (`self.ProjectileMovement`))
  (set `self.StartLocation` (`self.K2_GetActorLocation`)))

(event `self.StaticMesh.OnComponentHit`
  (params (HitComponent :type "PrimitiveComponent Object Reference") (OtherActor :type "Actor Object Reference") (OtherComp :type "PrimitiveComponent Object Reference") (NormalImpulse :type "Vector Structure") (Hit :type "HitResult Structure (by ref)"))
  (set `/Game/BetweenTheLines/Characters/SpiderCharacter/blueprints/BP_ThirdPersonSpider.GrappleStates` "NewEnumerator2" (`self.As BP Third Person Spider`))
  (set `self.HookedLocation` (`SceneComponent.K2_GetComponentLocation` (`self.Sphere`))))

(fn `GetArcPoints`
  (returns (ArcPointsO :type "Array of Vector Structure"))
  (return (`self.ArcPointsO`)))

(fn `UserConstructionScript`)