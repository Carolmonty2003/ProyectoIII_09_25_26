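; BP_Grappleable is an actor for the swing feature that decides whether an instigator can grapple it.
; CanGrapple measures the distance from the instigator's location to the hit's impact point.
; It refuses only when that distance is both below MinDistance and above MaxDistance, so it always allows grappling unless MinDistance exceeds MaxDistance.
; The event graph and construction script are empty.
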(fn `CanGrapple`
  (params (Instigator :type "Actor Object Reference") (Hit :type "HitResult Structure"))
  (returns (isGrappleable :type Boolean))
  (bind _returnvalue (`KismetMathLibrary.Vector_Distance` (`.ImpactPoint` (`GameplayStatics.BreakHitResult` Hit)) (`self.K2_GetActorLocation` Instigator)))
  (if (and (< _returnvalue (`self.MinDistance`)) (> _returnvalue (`self.MaxDistance`)))
    (return false)
    (else
      (return true))))

(fn `UserConstructionScript`)